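; BP_Character is a Gameplay Ability System character with mana regeneration, a resource bar widget and a Shocking Grasp melee hit.
; BeginPlay attaches MeleeSphere to a hand ability socket on the mesh, applies the regen effect and passes the AttributeSet to the widget.
; When MeleeSphere overlaps another BP_Character, it activates particles, applies a damage effect to that character and heals itself.
; An unconnected branch would remove the bar for the locally controlled player.
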(event OnComponentBeginOverlap(MeleeSphere)
  (params (OverlappedComponent :type Primitive%20Component%20Object%20Reference) (OtherActor :type Actor%20Object%20Reference) (OtherComp :type Primitive%20Component%20Object%20Reference) (OtherBodyIndex :type Integer) (bFromSweep :type Boolean) (SweepResult :type Hit%20Result%20Structure%20%28by%20ref%29))
  (bind _asbp_character (Utilities|Casting|CastToBP_Character OtherActor))
  (if (!= _asbp_character self)
    (Components|Activation|SetActive (Variables|Default|GetMeleeParticles) true false)
    (GameplayEffects|ApplyGameplayEffectToSelf :self (Variables|/Script/Arkde_MultiplayerGAS.Arkde_MultiplayerGASCharacter|GetAbilitySystemComponent _asbp_character) :GameplayEffectClass "/Game/Blueprints/Abilities/ShockingGrasp/GE_ShockingGrasp_Damage.GE_ShockingGrasp_Damage_C")
    (GameplayEffects|ApplyGameplayEffectToSelf :self (Variables|Default|GetAbilitySystemComponent) :GameplayEffectClass "/Game/Blueprints/Abilities/ShockingGrasp/GE_ShockingGrasp_Heal.GE_ShockingGrasp_Heal_C")))

(event EventBeginPlay
  (Transformation|AttachComponentToComponent (Variables|Default|GetMeleeSphere) (Variables|Character|GetMesh) "AbilityLeftSocket" "KeepRelative" "KeepRelative" "KeepRelative" true)
  (GameplayEffects|ApplyGameplayEffectToSelf :self (Variables|Default|GetAbilitySystemComponent) :GameplayEffectClass "/Game/Blueprints/Abilities/GE_Character_ManaRegen.GE_Character_ManaRegen_C")
  (bind _asw_resource_bars (Utilities|Casting|CastToW_ResourceBars (UserInterface|GetUserWidgetObject (Variables|Default|GetW_ResourceBar))))
  (Variables|/Game/Blueprints/UI/W_ResourceBars.W_ResourceBars_C|SetAttributeSet _asw_resource_bars (Variables|Default|GetAttributeSet)))

(event Collision|EventActorBeginOverlap
  (params (OtherActor :type Actor%20Object%20Reference)))

(event EventTick
  (params (DeltaSeconds :type Float%20%28single-precision%29)))

(fn ConstructionScript)