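; Gameplay ability for Shocking Grasp, a melee move that plays the AM_ShockingGrasp montage on the owning BP_Character once the ability commits.
; Montage notifies switch the character's MeleeSphere collision to query-only and back off, defining the hit window; hit handling is not in this graph.
; The ability ends when the montage completes, blends out or is interrupted, and OnEndAbility deactivates the character's MeleeParticles.
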(event Ability|EventActivateAbility
  (bind _asbp_character (Utilities|Casting|CastToBP_Character (Ability|GetOwningActorfromActorInfo)))
  (Variables|Default|SetCharacterReference _asbp_character)
  (bind _returnvalue (Ability|CommitAbility))
  (if _returnvalue
    (bind _notifyname (Animation|Montage|PlayMontage (Variables|/Script/Engine.Character|GetMesh (Variables|Default|GetCharacterReference)) "/Game/RetargetAnims/AM_ShockingGrasp.AM_ShockingGrasp" 0.8)
      (:OnCompleted
        (Ability|EndAbility :!label _label))
      (:OnBlendOut
        (goto _label))
      (:OnInterrupted
        (goto _label))
      (:OnNotifyBegin
        (switch name _notifyname
          (:ActivateCollision
            (Collision|SetCollisionEnabled (Variables|/Game/Blueprints/Character/BP_Character.BP_Character_C|GetMeleeSphere (Variables|Default|GetCharacterReference)) "QueryOnly"))
          (:DeactivateCollision
            (Collision|SetCollisionEnabled (Variables|/Game/Blueprints/Character/BP_Character.BP_Character_C|GetMeleeSphere (Variables|Default|GetCharacterReference)) "NoCollision")))))))

(event Ability|EventOnEndAbility
  (params (bWasCancelled :type Boolean))
  (Components|Activation|SetActive (Variables|/Game/Blueprints/Character/BP_Character.BP_Character_C|GetMeleeParticles (Variables|Default|GetCharacterReference)) false false))