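; Gameplay ability that casts a firebolt projectile from the owning BP_Character.
; After committing, it plays the cast montage and spawns BP_FireboltProjectile attached to the right ability socket, ignoring the caster when moving.
; A montage notify detaches the projectile and launches it along the character's forward vector at ProjectileSpeed.
; Montage completion, blend-out or interruption ends the ability, while a failed cast to BP_Character or failed commit cancels it.
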(event Ability|EventActivateAbility
  (bind _asbp_character (Utilities|Casting|CastToBP_Character (Ability|GetOwningActorfromActorInfo))
    (:then
      (Variables|Default|SetCharacterReference _asbp_character)
      (bind _returnvalue (Ability|CommitAbility))
      (if _returnvalue
        (Animation|Montage|PlayMontage (Variables|/Script/Engine.Character|GetMesh (Variables|Default|GetCharacterReference)) "/Game/RetargetAnims/AM_CastFirebolt.AM_CastFirebolt"
          (:then
            (bind _spawnedactor (|SpawnActor :Class "/Game/Blueprints/Abilities/Firebolt/BP_FireboltProjectile.BP_FireboltProjectile_C" :Instigator (Variables|Default|GetCharacterReference))
              (:Success
                (bind _asbp_firebolt_projectile (Utilities|Casting|CastToBP_FireboltProjectile _spawnedactor))
                (bind _output_get (Variables|Default|SetProjectileRef _asbp_firebolt_projectile))
                (Transformation|AttachActorToActor _output_get (Variables|Default|GetCharacterReference) "AbilityRightSocket" "KeepRelative" "KeepRelative" "KeepRelative" true)
                (Collision|IgnoreActorwhenMoving (Variables|/Script/Arkde_MultiplayerGAS.GAS_Projectile|GetSphereComponent (Variables|Default|GetProjectileRef)) (Variables|Default|GetCharacterReference) true))))
          (:OnCompleted
            (Ability|EndAbility :!label _label))
          (:OnBlendOut
            (goto _label))
          (:OnInterrupted
            (goto _label))
          (:OnNotifyBegin
            (bind _projectileref (Variables|Default|GetProjectileRef)
              (:then
                (Transformation|DetachFromActor _projectileref "KeepRelative" "KeepRelative" "KeepRelative")
                (Default|InitProjectileMovement (Variables|Default|GetProjectileRef) (* (Transformation|GetActorForwardVector (Variables|Default|GetCharacterReference)) (Variables|Default|GetProjectileSpeed))))
              (:else))))
        (else
          (Ability|CancelAbility :!label _label_2))))
    (:CastFailed
      (goto _label_2))))

(event Ability|EventOnEndAbility
  (params (bWasCancelled :type Boolean)))